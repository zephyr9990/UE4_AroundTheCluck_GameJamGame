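; Chicken AI character for Around The Cluck that lays eggs during the game's day cycle and can be kidnapped.
; Spawned-in chickens register with the GameMode, update the HUD count and sound an alarm between delays before initializing AI.
; GameMode cycle events start and stop a looping timer that spawns Egg_BP after random delays.
; Kidnapping toggles collision and a blackboard flag, with a panic sound on capture and a delayed reset on release.
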(event Custom|SetKidnapped
  (params (IsKidnapped :type Boolean))
  ;[1 1 1] Code that plays when chicken is kidnapped.
  (bind _output_get (Variables|Default|SetIsKidnapped IsKidnapped))
  (AI|Components|Blackboard|SetValueasBool (AI|GetBlackboard 0) (Variables|Default|GetIsBeingKidnapped) _output_get)
  (if _output_get
    (Collision|SetActorEnableCollision false)
    (Audio|PlaySoundatLocation "/Game/Audio/ChickenSound_Panic.ChickenSound_Panic" (Transformation|GetActorLocation) "0, 0, 0" 1.0 1.0 0.0 0 0 0)
    (else
      (Collision|SetActorEnableCollision true)
      (Transformation|SetActorRotation "0, 0, 0")
      (Utilities|FlowControl|Delay 1.0)
      (bind _output_get_2 (Variables|Default|SetIsKidnapped false))
      (AI|Components|Blackboard|SetValueasBool (AI|GetBlackboard 0) (Variables|Default|GetIsBeingKidnapped) _output_get_2))))

(event Custom|InitializeAIBehavior
  (bind _aroundthecluckgamemode (Variables|Default|GetAroundTheCluckGameMode))
  ;[1 1 1] Initializes AI Behavior
  (AI|Components|Blackboard|SetValueasObject (AI|GetBlackboard 0) (Variables|Default|GetBarnyardCenterPoint) (Variables|Default|GetBarnyardTargetPoint))
  (EventDispatchers|AssignStartDayTimeCycle _aroundthecluckgamemode (delegate Custom|StartHatchingEggs))
  (EventDispatchers|BindEventtoCycleTimeEnd _aroundthecluckgamemode (delegate Custom|StopHatchingEggs)))

(event Custom|StartHatchingEggs
  ;[1 1 1] Tell the chicken that they can start hatching eggs.
  (Variables|Default|SetCanHatchEgg true)
  (bind _returnvalue (Utilities|Time|SetTimerbyFunctionName self "HatchEggs" (/ 1.0 (Variables|Default|GetEggsPerSecond)) true))
  (Variables|Default|SetHatchEggsHandle _returnvalue))

(event Custom|HatchEggs
  (bind _returnvalue (Transformation|GetActorTransform))
  ;[1 1 1] Hatch an egg.
  (Utilities|FlowControl|Delay (Math|Random|RandomFloatinRange 0.0 (Variables|Default|GetMaxEggHatchDelayTime)))
  (if (Variables|Default|GetCanHatchEgg)
    (Game|SpawnActorfromClass "/Game/Blueprints/Pickups/Egg_BP.Egg_BP_C" (Math|Transform|MakeTransform (Math|Vector|MakeVector (.x (.location _returnvalue)) (.y (.location _returnvalue)) (Variables|Default|GetEggSpawnHeight))) "Undefined" 0 0)
    (Audio|PlaySoundatLocation "/Game/Audio/ChickenSound_ChickenClucking.ChickenSound_ChickenClucking" (Transformation|GetActorLocation) "0, 0, 0" 1.0 1.0 0.0 0 0 0)))

(event Custom|StopHatchingEggs
  (bind _hatcheggshandle (Variables|Default|GetHatchEggsHandle))
  ;[1 1 1] Stop hatching eggs.
  (if (Variables|Default|GetCanHatchEgg)
    (Variables|Default|SetCanHatchEgg false)
    (if (Utilities|Time|IsValidTimerHandle _hatcheggshandle)
      (Utilities|Time|ClearandInvalidateTimerbyHandle _hatcheggshandle))))

(event EventBeginPlay
  ;[1 1 1] BeginPlay
  (bind _asaround_the_cluck_game_mode_bp (Utilities|Casting|CastToAroundTheCluckGameMode_BP (Game|GetGameMode)))
  (bind _output_get (Variables|Default|SetAroundTheCluckGameMode _asaround_the_cluck_game_mode_bp))
  (if (not (Variables|Default|GetSpawnedIn))
    (CallFunction|InitializeAIBehavior)
    (else
      (Utilities|Array|Add (Variables|/Game/Blueprints/GameModes/AroundTheCluckGameMode_BP.AroundTheCluckGameMode_BP_C|GetChickens _output_get) self)
      (Default|UpdateRemainingChickens (Variables|/Game/Blueprints/GameModes/AroundTheCluckGameMode_BP.AroundTheCluckGameMode_BP_C|GetHUDRef _output_get) (Utilities|Array|Length (Variables|/Game/Blueprints/GameModes/AroundTheCluckGameMode_BP.AroundTheCluckGameMode_BP_C|GetChickens _output_get)))
      (Variables|Default|SetBarnyardTargetPoint (Variables|/Game/Blueprints/GameModes/AroundTheCluckGameMode_BP.AroundTheCluckGameMode_BP_C|GetBarnyardCenterPoint _output_get))
      (Utilities|FlowControl|Delay 5.0)
      (Audio|PlaySoundatLocation "/Game/Audio/ChickenSound_SingleAlarm.ChickenSound_SingleAlarm" (Transformation|GetActorLocation) "0, 0, 0" 1.0 1.0 0.0 0 0 0)
      (Utilities|FlowControl|Delay 5.0)
      (CallFunction|InitializeAIBehavior))))

(fn ConstructionScript)