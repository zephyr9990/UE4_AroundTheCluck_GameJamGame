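; Day/night lighting actor that fades a referenced GameLight between day and night looks as the game's cycle changes.
; On BeginPlay it binds ChangeLighting to AroundTheCluckGameMode_BP's CycleTimeEnd event and calls it once immediately.
; ChangeLighting plays IntensityTimeline forward when DayTime is true, otherwise reverses it.
; Timeline updates feed LerpLighting, which blends light intensity and color from day to night values.
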(event Custom|ChangeLighting
  ;[1 1 1] Switches lighting to the opposite lighting
  (if (Variables|/Game/Blueprints/GameModes/AroundTheCluckGameMode_BP.AroundTheCluckGameMode_BP_C|GetDayTime (Variables|Default|GetAroundTheCluckGameMode)) ; If it's currently daytime when cycle is switching...
    (bind _alpha (Timeline|IntensityTimeline Play)
      (:Update
        (Utilities|LerpLighting _alpha)))
    (else
      (Timeline|IntensityTimeline Reverse))))

(event EventBeginPlay
  (bind _asaround_the_cluck_game_mode_bp (Utilities|Casting|CastToAroundTheCluckGameMode_BP (Game|GetGameMode)))
  (bind _output_get (Variables|Default|SetAroundTheCluckGameMode _asaround_the_cluck_game_mode_bp))
  (EventDispatchers|AssignCycleTimeEnd _output_get (delegate Custom|ChangeLighting))
  (CallFunction|ChangeLighting))

(event Collision|EventActorBeginOverlap
  (params (OtherActor :type Actor%20Object%20Reference)))

(event EventTick
  (params (DeltaSeconds :type Float%20%28single-precision%29)))

(fn ConstructionScript)