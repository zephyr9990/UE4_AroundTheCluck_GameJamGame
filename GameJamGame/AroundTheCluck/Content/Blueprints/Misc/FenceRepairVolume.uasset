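; FenceRepairVolume is an actor marking a fence repair area that is active only during the day cycle.
; On BeginPlay it binds to the AroundTheCluck game mode's StartDayTimeCycle and CycleTimeEnd events to enable and disable repair.
; SetRepairEnabled toggles the widget's visibility and the actor's collision together.
; The construction script applies the configurable box extent and widget rotation.
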(event Custom|EnableRepair
  (Utilities|SetRepairEnabled true))

(event Custom|DisableRepair
  (Utilities|SetRepairEnabled false))

(event EventBeginPlay
  (bind _asaround_the_cluck_game_mode_bp (Utilities|Casting|CastToAroundTheCluckGameMode_BP (Game|GetGameMode)))
  (bind _output_get (Variables|Default|SetAroundTheCluckGameMode _asaround_the_cluck_game_mode_bp))
  (EventDispatchers|AssignStartDayTimeCycle _output_get (delegate Custom|EnableRepair))
  (EventDispatchers|AssignCycleTimeEnd _output_get (delegate Custom|DisableRepair)))

(event Collision|EventActorBeginOverlap
  (params (OtherActor :type Actor%20Object%20Reference)))

(event EventTick
  (params (DeltaSeconds :type Float%20%28single-precision%29)))

(fn ConstructionScript
  (Transformation|SetRelativeRotation (Variables|Default|GetWidget) (Variables|Default|GetWidgetRotation) false false)
  (Components|Box|SetBoxExtent (Variables|Default|GetRepairVolume) (Variables|Default|GetBoxExtent) true))