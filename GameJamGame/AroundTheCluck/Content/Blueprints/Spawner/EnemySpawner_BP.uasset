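; EnemySpawner_BP is a spawner actor that creates Wolf_BP AI enemies inside its spawn volume.
; BeginPlay caches the AroundTheCluck game mode, whose enemy count and cap gate each SpawnEnemy call.
; Each wolf spawns at a random point in the volume, gets the spawner's fence to attack and a random retreat point in the same volume, then increments the shared count.
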(event Custom|SpawnEnemy
  (bind _aroundthecluckgamemode (Variables|Default|GetAroundTheCluckGameMode))
  (bind _spawnvolume (Variables|Default|GetSpawnVolume))
  (bind _returnvalue (Transformation|GetWorldLocation _spawnvolume))
  (bind _returnvalue_2 (Components|Box|GetScaledBoxExtent _spawnvolume))
  (bind _returnvalue_3 (Math|Random|RandomPointinBoundingBox _returnvalue _returnvalue_2))
  ;[1 1 1] Spawn Enemy
  (if (< (Variables|/Game/Blueprints/GameModes/AroundTheCluckGameMode_BP.AroundTheCluckGameMode_BP_C|GetEnemyCount _aroundthecluckgamemode) (Variables|/Game/Blueprints/GameModes/AroundTheCluckGameMode_BP.AroundTheCluckGameMode_BP_C|GetMaxSpawnableEnemies _aroundthecluckgamemode))
    (bind _returnvalue_4 (AI|SpawnAIFromClass "/Game/Blueprints/Enemy/Wolf_BP.Wolf_BP_C" 0 _returnvalue_3 (Transformation|GetWorldRotation _spawnvolume) true))
    (bind _aswolf_bp (Utilities|Casting|CastToWolf_BP _returnvalue_4))
    (Default|SetFencetoAttack _aswolf_bp (Variables|Default|GetFenceToAttack))
    (Default|SetRetreatPoint _aswolf_bp _returnvalue_3)
    (Math|Integer|IncrementInt (Variables|/Game/Blueprints/GameModes/AroundTheCluckGameMode_BP.AroundTheCluckGameMode_BP_C|GetEnemyCount _aroundthecluckgamemode))))

(event EventBeginPlay
  ;[1 1 1] Stores game mode in variable.
  (bind _asaround_the_cluck_game_mode_bp (Utilities|Casting|CastToAroundTheCluckGameMode_BP (Game|GetGameMode)))
  (Variables|Default|SetAroundTheCluckGameMode _asaround_the_cluck_game_mode_bp))

(fn ConstructionScript)