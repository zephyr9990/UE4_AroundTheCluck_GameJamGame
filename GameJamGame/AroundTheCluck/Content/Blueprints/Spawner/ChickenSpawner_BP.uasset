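; Self-destroying spawner actor that brings in an AI chicken with an animated entrance and a choir sound.
; On BeginPlay, chained timelines scale the actor to its end size, rotate it in yaw, then reverse the scale before destroying it.
; In parallel, after a delay, it spawns Chicken_BP with its behavior tree from the Arrow's relative transform.
; A location timeline then moves the chicken vertically from the Arrow's world position to a fixed height.
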(event Custom|SpawnChicken
  (bind _arrow (Variables|Default|GetArrow))
  (bind _arrow_2 (Variables|Default|GetArrow))
  (bind _returnvalue (Transformation|GetRelativeTransform _arrow))
  (bind _returnvalue_2 (Transformation|GetWorldLocation _arrow_2))
  (bind (_x _y) (Math|Vector|BreakVector _returnvalue_2))
  ;[1 1 1] Spawns chicken
  (Utilities|FlowControl|Delay 3.0)
  (Audio|PlaySoundatLocation "/Game/Audio/ChoirSoundEffect.ChoirSoundEffect" "0, 0, 0" "0, 0, 0" 1.0 1.0 0.0 0 0 0)
  (bind _returnvalue_3 (AI|SpawnAIFromClass "/Game/Blueprints/Chicken/Chicken_BP.Chicken_BP_C" "/Game/Blueprints/Chicken/AI/Chicken_BehaviorTree.Chicken_BehaviorTree" (.location _returnvalue) (.rotation _returnvalue) false))
  (bind _aschicken_bp (Utilities|Casting|CastToChicken_BP _returnvalue_3))
  (bind _output_get (Variables|Default|SetSpawnedChicken _aschicken_bp))
  (bind _alpha (Timeline|LocationTimeline Play)
    (:Update
      (Transformation|SetActorLocation _output_get (Math|Vector|Lerp(Vector) _returnvalue_2 (Math|Vector|MakeVector _x _y 144.0) _alpha) false false))))

(event EventBeginPlay
  ;[1 1 1] Begin play
  (CallFunction|SpawnChicken)
  (bind (_direction _alpha) (Timeline|ScaleTimeline Play)
    (:Update
      (Transformation|SetActorScale3D (Math|Vector|Lerp(Vector) "0, 0,100.000000" (Variables|Default|GetEndScaleSize) _alpha)))
    (:Finished
      (if (Utilities|Enum|Equal(Enum) _direction "Forward")
        (bind _alpha_2 (Timeline|RotationTimeLine Play)
          (:Update
            (Transformation|SetActorRotation (Math|Rotator|Lerp(Rotator) (Transformation|GetActorRotation) (Math|Rotator|MakeRotator 0.0 0.0 (Variables|Default|GetDesiredEndRotation)) _alpha_2)))
          (:Finished
            (Timeline|ScaleTimeline Reverse)))
        (else
          (Actor|DestroyActor))))))

(fn ConstructionScript)