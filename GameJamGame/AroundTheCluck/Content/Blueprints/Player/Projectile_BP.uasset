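; Player projectile Blueprint that damages enemies it overlaps.
; On sphere overlap it acts only on actors that implement IDamageable and carry the enemy tag.
; A valid hit spawns a spark emitter at its XY but at WolfHeight, plays a random impact sound, sends the damage message to the target and destroys the projectile.
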(event OnComponentBeginOverlap(SphereCollision)
  (params (OverlappedComponent :type Primitive%20Component%20Object%20Reference) (OtherActor :type Actor%20Object%20Reference) (OtherComp :type Primitive%20Component%20Object%20Reference) (OtherBodyIndex :type Integer) (bFromSweep :type Boolean) (SweepResult :type Hit%20Result%20Structure%20%28by%20ref%29))
  (bind _returnvalue (Transformation|GetActorTransform))
  (bind _impactsounds (Variables|Default|GetImpactSounds))
  (if (and (Utilities|DoesObjectImplementInterface OtherActor "/Game/Blueprints/Interfaces/IDamageable.IDamageable_C") (Actor|ActorHasTag OtherActor (Variables|Default|GetEnemyTag)))
    (Effects|SpawnEmitteratLocation "/Game/VFX/P_MySparks.P_MySparks" (Math|Vector|MakeVector (.x (.location _returnvalue)) (.y (.location _returnvalue)) (Variables|Default|GetWolfHeight)) (.rotation _returnvalue))
    (Audio|SpawnSoundatLocation (Utilities|Array|Get(acopy) _impactsounds (Math|Random|RandomInteger (Utilities|Array|Length _impactsounds))) (Math|Vector|MakeVector (.x (.location _returnvalue)) (.y (.location _returnvalue)) (.z (.location _returnvalue))) "0, 0, 0" 1.0 1.0 0.0 0 0)
    (Class|IDamageable|TakeDamage(Message) OtherActor (Variables|Default|GetProjectileDamage))
    (Actor|DestroyActor)))

(fn ConstructionScript)