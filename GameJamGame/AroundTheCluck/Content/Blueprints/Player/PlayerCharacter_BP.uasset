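; Player character for Around The Cluck that clamps its spring-arm camera each tick, owns the player HUD and repairs fences.
; Game mode day-cycle events switch fence repair on and off.
; Overlapping a damaged fence's repair volume swaps gun for hammer and loops the montage on a timer.
; The anim Blueprint calls RepairFence to apply repair through TakeDamage; hammering stops at full health or when leaving the volume.
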(event Custom|ToggleHUDOn
  ;[1 1 1] Toggle HUD
  (UserInterface|Viewport|AddtoViewport (Variables|Default|GetHUDRef) 0))

(event Custom|ToggleHUDOff
  ;[1 1 1] Toggle HUD
  (Widget|RemovefromParent (Variables|Default|GetHUDRef)))

(event Custom|EnableFenceRepair
  ;[1 1 1] Set whether the player can repair fences.
  (Variables|Default|SetCanRepairFence true))

(event Custom|HammerFence
  (bind _fencetorepair (Variables|Default|GetFenceToRepair))
  ;[1 1 1] Repair Fence
  ;;[1 1 1] Plays repair montage
  (if (>= (Variables|/Game/Blueprints/Misc/Fence_BP.Fence_BP_C|GetCurrentHealth _fencetorepair) (Variables|/Game/Blueprints/Misc/Fence_BP.Fence_BP_C|GetMaxHealth _fencetorepair))
    (Utilities|StopHammering)
    (else
      (Animation|PlayAnimMontage "/Game/Animations/Player/Hammer_Montage.Hammer_Montage" 1.0 "None"))))

(event Custom|RepairFence
  (bind _fencetorepair (Variables|Default|GetFenceToRepair))
  ;[1 1 1] Repair Fence
  ;;[1 1 1] Repairs fence, called from anim BP
  (Utilities|IsValid _fencetorepair
    (:Is%20Valid
      (Default|TakeDamage _fencetorepair (Variables|Default|GetRepairAmount))
      (if (>= (Variables|/Game/Blueprints/Misc/Fence_BP.Fence_BP_C|GetCurrentHealth _fencetorepair) (Variables|/Game/Blueprints/Misc/Fence_BP.Fence_BP_C|GetMaxHealth _fencetorepair))
        (Default|DisableRepair (Variables|Default|GetFenceRepairVolume))))))

(event Custom|DisableFenceRepair
  ;[1 1 1] Set whether the player can repair fences.
  (Variables|Default|SetCanRepairFence false))

(event EventBeginPlay
  ;[1 1 1] Add Player HUD to screen.
  (Variables|Default|SetCameraDefaultRelativeLocation (Variables|/Script/Engine.SceneComponent|GetRelativeLocation (Variables|Default|GetCamera)))
  (bind _returnvalue (UserInterface|CreateWidget "/Game/UI/Blueprints/PlayerHUD_BP.PlayerHUD_BP_C" (Game|GetPlayerController 0)))
  (bind _output_get (Variables|Default|SetHUDRef _returnvalue))
  (UserInterface|Viewport|AddtoViewport _output_get 0)
  (bind _asaround_the_cluck_game_mode_bp (Utilities|Casting|CastToAroundTheCluckGameMode_BP (Game|GetGameMode)))
  (bind _output_get_2 (Variables|Default|SetAroundTheCluckGameMode _asaround_the_cluck_game_mode_bp))
  (Default|SetHUDRef _output_get_2 _output_get)
  (Default|UpdateRemainingChickens (Variables|Default|GetHUDRef) (Utilities|Array|Length (Variables|/Game/Blueprints/GameModes/AroundTheCluckGameMode_BP.AroundTheCluckGameMode_BP_C|GetChickens _output_get_2)))
  (EventDispatchers|AssignStartDayTimeCycle _output_get_2 (delegate Custom|EnableFenceRepair))
  (EventDispatchers|BindEventtoCycleTimeEnd _output_get_2 (delegate Custom|DisableFenceRepair)))

(event Collision|EventActorBeginOverlap
  (params (OtherActor :type Actor%20Object%20Reference))
  ;[1 1 1] Repair Fence
  (if (Variables|Default|GetCanRepairFence)
    (bind _asfence_repair_volume (Utilities|Casting|CastToFenceRepairVolume OtherActor))
    (Variables|Default|SetFenceRepairVolume _asfence_repair_volume)
    (Utilities|IsValid (Variables|/Game/Blueprints/Misc/FenceRepairVolume.FenceRepairVolume_C|GetFenceToRepair _asfence_repair_volume)
      (:Is%20Valid
        (if (and (Actor|ActorHasTag OtherActor (Variables|Default|GetFenceRepairTag)) (< (Variables|/Game/Blueprints/Misc/Fence_BP.Fence_BP_C|GetCurrentHealth (Variables|/Game/Blueprints/Misc/FenceRepairVolume.FenceRepairVolume_C|GetFenceToRepair _asfence_repair_volume)) (Variables|/Game/Blueprints/Misc/Fence_BP.Fence_BP_C|GetMaxHealth (Variables|/Game/Blueprints/Misc/FenceRepairVolume.FenceRepairVolume_C|GetFenceToRepair _asfence_repair_volume)))) ; If actor is a fence repair volume, and fence needs repair...
          (Variables|Default|SetFenceToRepair (Variables|/Game/Blueprints/Misc/FenceRepairVolume.FenceRepairVolume_C|GetFenceToRepair _asfence_repair_volume))
          (CallFunction|HammerFence)
          (bind _returnvalue (Animation|GetPlayLength (Variables|Default|GetHammerMontage)))
          (Utilities|Time|SetTimerbyFunctionName 0 (Variables|Default|GetHammerFenceFunctionName) _returnvalue true)
          (Utilities|ShowHammer true))))))

(event Collision|EventActorEndOverlap
  (params (OtherActor :type Actor%20Object%20Reference))
  ;[1 1 1] Repair Fence
  (Utilities|IsValid OtherActor
    (:Is%20Valid
      (if (Actor|ActorHasTag OtherActor (Variables|Default|GetFenceRepairTag))
        (Utilities|StopHammering)))))

(event EventTick
  (params (DeltaSeconds :type Float%20%28single-precision%29))
  (Class|PlayerCharacter|ClampCamera (Variables|Default|GetSpringArm)))

(fn ConstructionScript)