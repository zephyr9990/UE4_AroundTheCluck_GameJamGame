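; Player controller that toggles the pause menu when the Pause input is pressed.
; Pausing creates and shows PauseMenu_BP, switches to game-and-UI input with the cursor visible, pauses the game and hides the player character's HUD.
; Unpausing, reached by pressing again while the menu exists or through the Unpause event, removes the menu and restores game-only input, play and HUD.
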(event Custom|Unpause
  ;[1 1 1] Pause/Unpause game.
  (Widget|RemovefromParent (Variables|Default|GetPauseMenuRef))
  (Variables|Default|SetPauseMenuRef 0)
  (Input|SetInputModeGameOnly (Game|GetPlayerController 0))
  (Variables|Default|SetbShowMouseCursor false)
  (Game|SetGamePaused false)
  (Default|ToggleHUDon (.AsPlayer%20Character%20BP (Utilities|Casting|CastToPlayerCharacter_BP (Game|GetPlayerCharacter 0)))))

(event Input|ActionEvents|InputActionPause
  (params (Key :type Key%20Structure))
  ;[1 1 1] Pause/Unpause game.
  (:Pressed
    (Utilities|IsValid (Variables|Default|GetPauseMenuRef)
      (:Is%20Valid
        (Widget|RemovefromParent (Variables|Default|GetPauseMenuRef))
        (Variables|Default|SetPauseMenuRef 0)
        (Input|SetInputModeGameOnly (Game|GetPlayerController 0))
        (Variables|Default|SetbShowMouseCursor false)
        (Game|SetGamePaused false)
        (Default|ToggleHUDon (.AsPlayer%20Character%20BP (Utilities|Casting|CastToPlayerCharacter_BP (Game|GetPlayerCharacter 0)))))
      (:Is%20Not%20Valid
        (bind _returnvalue (UserInterface|CreateWidget "/Game/UI/Blueprints/PauseMenu_BP.PauseMenu_BP_C"))
        (bind _output_get (Variables|Default|SetPauseMenuRef _returnvalue))
        (UserInterface|Viewport|AddtoViewport _output_get 0)
        (Input|SetInputModeGameandUI (Game|GetPlayerController 0) 0 "DoNotLock" true)
        (Variables|Default|SetbShowMouseCursor true)
        (Game|SetGamePaused true)
        (Default|ToggleHUDOff (.AsPlayer%20Character%20BP (Utilities|Casting|CastToPlayerCharacter_BP (Game|GetPlayerCharacter 0))))))))

(fn ConstructionScript)