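; Player gun Blueprint that supplies the gun's colored body, projectile spawn point and muzzle flash effect.
; The construction script creates a dynamic material on the gun mesh, tints it with GunColor and stores the ProjectileSpawn component as ProjectileSpawnPoint.
; ShowMuzzleFlash briefly shows the MuzzleFlash component and spawns a spark emitter attached at the projectile spawn, hiding the flash again after a short delay.
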(event EventShowMuzzleFlash
  (bind _muzzleflash (Variables|Default|GetMuzzleFlash))
  (bind _projectilespawn (Variables|Default|GetProjectileSpawn))
  (bind _returnvalue (Transformation|GetWorldTransform _projectilespawn))
  ;[1 1 1] Play muzzle flash effects
  (Rendering|SetVisibility _muzzleflash true false)
  (Effects|SpawnEmitterAttached "/Game/VFX/P_MuzzleSparks.P_MuzzleSparks" _projectilespawn "None" (.location _returnvalue) (.rotation _returnvalue) "1.000000,1.000000,1.000000" "KeepWorldPosition")
  (Utilities|FlowControl|Delay 0.2)
  (Rendering|SetVisibility _muzzleflash false false))

(fn ConstructionScript
  (bind _returnvalue (Rendering|Material|CreateDynamicMaterialInstance (Variables|Default|GetGunMesh) 0 0 "BodyColor" :!class /Script/Engine.PrimitiveComponent))
  (bind _output_get (Variables|Default|SetDynamicMaterial _returnvalue))
  (Rendering|Material|SetVectorParameterValue _output_get "BodyColor" (Variables|Default|GetGunColor) :!class /Script/Engine.MaterialInstanceDynamic)
  (Variables|Default|SetProjectileSpawnPoint (Variables|Default|GetProjectileSpawn)))