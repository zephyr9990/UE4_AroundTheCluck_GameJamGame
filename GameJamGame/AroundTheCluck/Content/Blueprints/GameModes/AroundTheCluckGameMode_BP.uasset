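; Game mode for Around the Cluck, running alternating day and night cycles in which chickens face kidnapping by wolves.
; Looping timers drive the countdown and, at night, random-spawner enemy spawns, while event dispatchers announce cycle and chicken state changes.
; It tracks score, eggs and chickens, pushing updates to the HUD.
; Enough eggs spawn a chicken spawner above the player; losing every chicken pauses into game over.
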(event Custom|StartNightTime
  ;[1 1 1] Start night time.
  (Audio|PlaySound2D "/Game/Audio/WolfSound_Howl.WolfSound_Howl" 1.0 1.0 0.0 0 0)
  (bind _returnvalue (Utilities|Time|SetTimerbyFunctionName 0 "DecrementTimer" 1.0 true))
  (Variables|Default|SetDecrementTimerHandle _returnvalue)
  (bind _returnvalue_2 (Utilities|Time|SetTimerbyFunctionName self "SpawnEnemies" (/ 1.0 (Variables|Default|GetEnemiesSpawningPerSecond)) true))
  (Variables|Default|SetSpawnEnemiesHandle _returnvalue_2)
  (Default|UpdateTimeCycle (Variables|Default|GetHUDRef) (Variables|Default|GetDayTime))
  (Default|CallStartNightTimeCycle))

(event Custom|SpawnEnemies
  (bind _enemyspawners (Variables|Default|GetEnemySpawners))
  ;[1 1 1] Spawns an enemy by randomly picking a spawner to spawn an enemy from.
  (Default|SpawnEnemy (Utilities|Array|Get(acopy) _enemyspawners (Math|Random|RandomInteger (Utilities|Array|Length _enemyspawners)))))

(event Custom|GameOver
  (bind _returnvalue (Game|GetPlayerController 0))
  ;[1 1 1] Game over event.
  (Utilities|FlowControl|Delay 0.5)
  (bind _returnvalue_2 (UserInterface|CreateWidget "/Game/UI/Blueprints/GameOver_BP.GameOver_BP_C"))
  (UserInterface|Viewport|AddtoViewport _returnvalue_2 0)
  (Input|SetInputModeUIOnly _returnvalue 0 "DoNotLock")
  (Variables|/Script/Engine.PlayerController|SetbShowMouseCursor _returnvalue true)
  (Game|SetGamePaused true)
  (Default|ToggleHUDOff (.AsPlayer%20Character%20BP (Utilities|Casting|CastToPlayerCharacter_BP (Game|GetPlayerCharacter 0)))))

(event Custom|SetHUDRef
  (params (HUDRef :type Player%20HUD%20BP%20Object%20Reference))
  ;[1 1 1] Set HUD reference.
  (Variables|Default|SetHUDRef HUDRef))

(event Custom|DecrementTimer
  (bind _currentcycletime (Variables|Default|GetCurrentCycleTime))
  ;[1 1 1] Decrement time remaining in cycle.
  (bind _result (Math|Float|DecrementFloat _currentcycletime)
    (:%20%20
      (Default|UpdateTimeRemaining (Variables|Default|GetHUDRef) _result)
      (if (<= _currentcycletime 0.0)
        (Default|CallCycleTimeEnd)
        (CallFunction|SwitchCycle)))))

(event Custom|ChickenWasKidnapped
  ;[1 1 1] Chicken was either kidnapped or released. Tell all wolves subscribed to see if they need to target another chicken.
  (Default|CallChickenStateChanged))

(event Custom|ChickenWasReleased
  ;[1 1 1] Chicken was either kidnapped or released. Tell all wolves subscribed to see if they need to target another chicken.
  (Default|CallChickenStateChanged))

(event Custom|AddScore
  (params (Score :type Integer))
  ;[1 1 1] Adds to player score
  (bind _output_get (Variables|Default|SetPlayerScore (+ Score (Variables|Default|GetPlayerScore))))
  (Default|UpdateScore (Variables|Default|GetHUDRef) _output_get))

(event Custom|SwitchCycle
  (bind _cyclechangedelay (Variables|Default|GetCycleChangeDelay))
  ;[1 1 1] Switches the current cycle
  (Utilities|ClearTimers)
  (Variables|Default|SetCurrentCycleTime (Variables|Default|GetDefaultCycleTime))
  (bind _output_get (Variables|Default|SetDayTime (not (Variables|Default|GetDayTime))))
  (if _output_get ; If day time...
    (Default|UpdateCycleDelayText (Variables|Default|GetHUDRef) (Variables|Default|GetDayTime))
    (Utilities|FlowControl|Delay _cyclechangedelay)
    (CallFunction|StartDayTime)
    (else
      (Default|UpdateCycleDelayText (Variables|Default|GetHUDRef) (Variables|Default|GetDayTime))
      (Utilities|FlowControl|Delay _cyclechangedelay)
      (CallFunction|StartNightTime))))

(event Custom|StartDayTime
  ;[1 1 1] Start Day Time
  (Audio|PlaySound2D "/Game/Audio/ChickenSound_RoosterCrow.ChickenSound_RoosterCrow" 1.0 1.0 0.0 0 0)
  (bind _returnvalue (Utilities|Time|SetTimerbyFunctionName 0 "DecrementTimer" 1.0 true))
  (Variables|Default|SetDecrementTimerHandle _returnvalue)
  (Default|UpdateTimeCycle (Variables|Default|GetHUDRef) (Variables|Default|GetDayTime))
  (Default|CallStartDayTimeCycle))

(event Custom|AddEggs
  (params (Eggs :type Integer))
  (bind _returnvalue (Game|GetPlayerCharacter 0))
  (bind _returnvalue_2 (Transformation|GetActorTransform _returnvalue))
  ;[1 1 1] Add eggs and update player HUD
  (Variables|Default|SetCurrentEggCount (+ Eggs (Variables|Default|GetCurrentEggCount)))
  (if (== (Variables|Default|GetCurrentEggCount) (Variables|Default|GetNumEggsRequiredToSpawnChicken))
    (Variables|Default|SetCurrentEggCount 0)
    (Game|SpawnActorfromClass "/Game/Blueprints/Spawner/ChickenSpawner_BP.ChickenSpawner_BP_C" (Math|Transform|MakeTransform (Math|Vector|MakeVector (.x (.location _returnvalue_2)) (.y (.location _returnvalue_2)) (Variables|Default|GetChickenSpawnerSpawnHeight)) "0, 0, 0" "1,1,1") "Undefined" 0 0))
  (Default|UpdateEggCount (Variables|Default|GetHUDRef) (Variables|Default|GetCurrentEggCount)))

(event EventBeginPlay
  ;[1 1 1] Start appropriate game play based on time.
  (bind _outactors (Actor|GetAllActorsOfClass "/Game/Blueprints/Spawner/EnemySpawner_BP.EnemySpawner_BP_C"))
  (Variables|Default|SetEnemySpawners _outactors)
  (bind _outactors_2 (Actor|GetAllActorsOfClass "/Script/Engine.TargetPoint"))
  (Variables|Default|SetBarnyardCenterPoint (Utilities|Array|Get(acopy) _outactors_2))
  (Utilities|GetAllChickens)
  (Utilities|FlowControl|Delay 0.2)
  (CallFunction|SwitchCycle))

(fn ConstructionScript)

(fn RemoveChicken
  (params (KidnappedChicken :type Chicken%20BP%20Object%20Reference))
  (bind _chickens (Variables|Default|GetChickens))
  (bind _returnvalue (Utilities|Array|Length _chickens))
  ;[1 1 1] Decrements chickens when kidnapped and calls game over when count is 0.
  (Utilities|Array|RemoveItem _chickens KidnappedChicken)
  (bind _asplayer_character_bp (Utilities|Casting|CastToPlayerCharacter_BP (Game|GetPlayerCharacter 0)))
  (Default|UpdateRemainingChickens (Variables|/Game/Blueprints/Player/PlayerCharacter_BP.PlayerCharacter_BP_C|GetHUDRef _asplayer_character_bp) _returnvalue)
  (if (<= _returnvalue 0)
    (CallFunction|GameOver)))